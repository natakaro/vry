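; Menu block actor that opens ExampleMap when the player triggers one of its two meshes.
; Each tick it polls StaticMesh and Cube for any overlapping actor, then checks the SculptSingle flag on the player's MotionControllerPawn2.
; If the flag is set, it loads the level, passing a different Variable value in the options string for each mesh.
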(event `self.ReceiveTick`
  (params (DeltaSeconds :type "Float (single-precision)"))
  (`|ExecutionSequence`
    (:`then_0`
      (if (> (`KismetArrayLibrary.Array_Length` (`PrimitiveComponent.GetOverlappingActors` (`self.StaticMesh`) null)) 0)
        (bind _asmotion_controller_pawn_2 (cast `/Game/Proteus_Single/Blueprints/MotionControllerPawn2` (`GameplayStatics.GetPlayerPawn` 0)))
        (if (`/Game/Proteus_Single/Blueprints/MotionControllerPawn2.sculptSingle` _asmotion_controller_pawn_2)
          (`GameplayStatics.OpenLevel` "ExampleMap" true "?Variable=100"))))
    (:`then_1`
      (if (> (`KismetArrayLibrary.Array_Length` (`PrimitiveComponent.GetOverlappingActors` (`self.Cube`) null)) 0)
        (bind _asmotion_controller_pawn_2_2 (cast `/Game/Proteus_Single/Blueprints/MotionControllerPawn2` (`GameplayStatics.GetPlayerPawn` 0)))
        (if (`/Game/Proteus_Single/Blueprints/MotionControllerPawn2.sculptSingle` _asmotion_controller_pawn_2_2)
          (`GameplayStatics.OpenLevel` "ExampleMap" true "?Variable=1"))))))

(fn `UserConstructionScript`)