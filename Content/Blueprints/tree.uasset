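; A VR tree actor that can be picked up, dropped and planted on terrain.
; Pickup, called by the motion controller, works only while a VR HUD reference is valid: it stops physics, attaches the tree and tells the HUD to spawn a tree.
; Drop re-enables physics, detaches and clears that reference.
; Hitting a terrain section snaps the mesh to the impact point and freezes physics, with a leftover debug print.
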(event `/Game/Proteus_Single/Blueprints/PickupActorInterface.Pickup`
  (params (AttachTo :type "SceneComponent Object Reference"))
  (bind _vrhud (`self.VRhud`))
  (if (`KismetSystemLibrary.IsValid` _vrhud)
    (`PrimitiveComponent.SetSimulatePhysics` (`self.StaticMesh`) false)
    (`self.K2_DetachFromActor` "KeepWorld" "KeepWorld" "KeepWorld")
    (`SceneComponent.K2_AttachToComponent` (`self.K2_GetRootComponent`) AttachTo "None" "SnapToTarget" "SnapToTarget" "KeepWorld" false)
    (`/Game/Blueprints/VRhud.SpawnTree` _vrhud)))

(event `/Game/Proteus_Single/Blueprints/PickupActorInterface.Drop`
  (`PrimitiveComponent.SetSimulatePhysics` (`self.StaticMesh`) true)
  (`self.K2_DetachFromActor` "KeepWorld" "KeepWorld" "KeepWorld")
  (set `self.VRhud` null))

(event `self.StaticMesh.OnComponentHit`
  (params (HitComponent :type "PrimitiveComponent Object Reference") (OtherActor :type "Actor Object Reference") (OtherComp :type "PrimitiveComponent Object Reference") (NormalImpulse :type "Vector Structure") (Hit :type "HitResult Structure (by ref)"))
  (bind _staticmesh (`self.StaticMesh`))
  (cast `/Game/Blueprints/BP_MyTerrainSection` OtherActor)
  (`KismetSystemLibrary.PrintString` "Hello")
  (`SceneComponent.K2_SetWorldLocationAndRotation` :`self` _staticmesh :`NewLocation` (`.ImpactPoint` (`GameplayStatics.BreakHitResult` Hit)))
  (`PrimitiveComponent.SetSimulatePhysics` _staticmesh false))

(fn `UserConstructionScript`)