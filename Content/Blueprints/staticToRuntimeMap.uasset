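; Actor Blueprint that turns a static mesh into a runtime mesh.
; The construction script copies the StaticMesh component into the RuntimeMesh component with collision enabled, then destroys the StaticMesh component.
; The event graph does no work; disconnected nodes that build a hand-made quad mesh section remain in both graphs but never run.
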(fn `UserConstructionScript`
  (`RuntimeMeshLibrary.CopyRuntimeMeshFromStaticMeshComponent` (`self.StaticMesh`) 0 (`self.RuntimeMesh`) true)
  (`ActorComponent.K2_DestroyComponent` (`self.StaticMesh`)))