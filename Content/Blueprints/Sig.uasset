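; Sig is a VR signal object that the player picks up with a motion controller and drops or throws onto terrain.
; Pickup disables physics and snaps it to the hand if the VR HUD is valid, while dropping restores physics and starts a short timer.
; Hitting a terrain section freezes it at the impact point, otherwise the timer destroys it.
; On destruction it asks the VR HUD to spawn a signal.
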(event `self.Sphere1.OnComponentBeginOverlap`
  (params (OverlappedComponent :type "PrimitiveComponent Object Reference") (OtherActor :type "Actor Object Reference") (OtherComp :type "PrimitiveComponent Object Reference") (OtherBodyIndex :type Integer) (bFromSweep :type Boolean) (SweepResult :type "HitResult Structure (by ref)")))

(event `/Game/Proteus_Single/Blueprints/PickupActorInterface.Pickup`
  (params (AttachTo :type "SceneComponent Object Reference"))
  (if (`KismetSystemLibrary.IsValid` (`self.VRhud`))
    (`PrimitiveComponent.SetSimulatePhysics` (`self.Sphere`) false)
    (`self.K2_DetachFromActor` "KeepWorld" "KeepWorld" "KeepWorld")
    (`SceneComponent.K2_AttachToComponent` (`self.K2_GetRootComponent`) AttachTo "None" "SnapToTarget" "SnapToTarget" "KeepWorld" false)))

(event `/Game/Proteus_Single/Blueprints/PickupActorInterface.Drop`
  (`PrimitiveComponent.SetSimulatePhysics` (`self.Sphere`) true)
  (`self.K2_DetachFromActor` "KeepWorld" "KeepWorld" "KeepWorld")
  (`self.Timer`))

(event `self.Sphere.OnComponentHit`
  (params (HitComponent :type "PrimitiveComponent Object Reference") (OtherActor :type "Actor Object Reference") (OtherComp :type "PrimitiveComponent Object Reference") (NormalImpulse :type "Vector Structure") (Hit :type "HitResult Structure (by ref)"))
  (bind _sphere (`self.Sphere`))
  (cast `/Game/Blueprints/BP_MyTerrainSection` OtherActor)
  (`SceneComponent.K2_SetWorldLocationAndRotation` :`self` _sphere :`NewLocation` (`.ImpactPoint` (`GameplayStatics.BreakHitResult` Hit)))
  (`PrimitiveComponent.SetSimulatePhysics` _sphere false)
  (set `self.spawned` true))

(event `Timer`
  (`KismetSystemLibrary.Delay` 3.0)
  (if (not (`self.spawned`))
    (`self.K2_DestroyActor`)))

(event `self.ReceiveDestroyed`
  (`/Game/Blueprints/VRhud.SpawnSignal` (`self.VRhud`)))

(fn `DestroyME`
  (if (`self.spawned`)
    (`self.K2_DestroyActor`)))

(fn `UserConstructionScript`)