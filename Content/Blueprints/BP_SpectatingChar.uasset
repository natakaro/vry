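; Free-flying spectator character that sculpts via a Sculpt component and shows a brush decal under the cursor.
; Axis inputs move it along the control rotation, the mouse wheel adjusts fly speed, and holding left mouse sculpts while locking camera look.
; Tick feeds the cursor trace to Sculpt, then positions and sizes the decal from the sculpt radius and falloff.
; BeginPlay creates the HUD linked to Sculpt and the decal's dynamic material.
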(event `InputAxis|Turn`
  (params (AxisValue :type "Float (single-precision)"))
  ;[1 1 1] Camera
  (if (not (`self.DisableCameraMovement`))
    (`self.AddControllerYawInput` AxisValue)))

(event `InputAxis|LookUp`
  (params (AxisValue :type "Float (single-precision)"))
  ;[1 1 1] Camera
  (if (not (`self.DisableCameraMovement`))
    (`self.AddControllerPitchInput` AxisValue)))

(event `InputAxis|MoveForward`
  (params (AxisValue :type "Float (single-precision)"))
  ;[1 1 1] Movement
  (`self.AddMovementInput` (`KismetMathLibrary.GetForwardVector` (`self.GetControlRotation`)) AxisValue))

(event `InputAxis|MoveRight`
  (params (AxisValue :type "Float (single-precision)"))
  ;[1 1 1] Movement
  (`self.AddMovementInput` (`KismetMathLibrary.GetRightVector` (`self.GetControlRotation`)) AxisValue))

(event `InputAxis|MoveUp`
  (params (AxisValue :type "Float (single-precision)"))
  (bind (_returnvalue_roll _returnvalue_pitch _returnvalue_yaw) (`KismetMathLibrary.BreakRotator` (`self.GetControlRotation`)))
  ;[1 1 1] Movement
  (`self.AddMovementInput` (`KismetMathLibrary.GetUpVector` (`KismetMathLibrary.MakeRotator` 0.0 0.0 _returnvalue_yaw)) AxisValue))

(event `Key|MouseScrollUp`
  (params (Key :type "Key Structure" :default "AnyKey"))
  (bind _charactermovement (`self.CharacterMovement`))
  (bind _returnvalue (`KismetMathLibrary.FClamp` (+ (`CharacterMovementComponent.MaxFlySpeed` _charactermovement) 1000.0) 1000.0 100000.0))
  ;[1 1 1] Change Fly Speed
  (:`Pressed`
    (set `CharacterMovementComponent.MaxFlySpeed` _returnvalue _charactermovement)
    (set `CharacterMovementComponent.MaxAcceleration` _returnvalue _charactermovement)))

(event `Key|MouseScrollDown`
  (params (Key :type "Key Structure" :default "AnyKey"))
  (bind _charactermovement (`self.CharacterMovement`))
  (bind _returnvalue (`KismetMathLibrary.FClamp` (- (`CharacterMovementComponent.MaxFlySpeed` _charactermovement) 1000.0) 1000.0 100000.0))
  ;[1 1 1] Change Fly Speed
  (:`Pressed`
    (set `CharacterMovementComponent.MaxFlySpeed` _returnvalue _charactermovement)
    (set `CharacterMovementComponent.MaxAcceleration` _returnvalue _charactermovement)))

(event `Key|LeftMouseButton`
  (params (Key :type "Key Structure" :default "AnyKey"))
  (:`Pressed`
    ;[1 1 1] Sculpt
    (`SculptComponent.SculptStart` (`self.Sculpt`)))
  (:`Released`
    (`SculptComponent.SculptStop` (`self.Sculpt`))))

(event `InputAction|LMB`
  (params (Key :type "Key Structure" :default "AnyKey"))
  ;[1 1 1] LMB
  (:`Pressed`
    (set `self.LMBDown` true)
    (set `self.DisableCameraMovement` true))
  (:`Released`
    (bind _output_get (set `self.LMBDown` false))
    (`KismetSystemLibrary.Delay` 0.05)
    (if (not _output_get)
      (set `self.DisableCameraMovement` false))))

(event `self.ReceiveBeginPlay`
  (bind _returnvalue (`GameplayStatics.GetPlayerController` 0))
  ;[1 1 1] begin play
  ;;[1 1 1] Create HUD and set game mode
  (bind _returnvalue_2 (`|CreateWidget` "/Game/Blueprints/WBP_HUD.WBP_HUD_C" null (`self.Sculpt`) 5000.0 1000.0))
  (`UserWidget.AddToViewport` _returnvalue_2 0)
  (set `self.HUDRef` _returnvalue_2)
  (`WidgetBlueprintLibrary.SetInputMode_GameAndUIEx` _returnvalue _returnvalue_2 "DoNotLock" false)
  (set `PlayerController.bShowMouseCursor` true _returnvalue)
  ;;[1 1 1] dynamic material instance for brush decal
  (bind _returnvalue_3 (`KismetMaterialLibrary.CreateDynamicMaterialInstance` "/Game/Materials/MI_DecalBrush.MI_DecalBrush"))
  (set `self.DecalMatInstance` _returnvalue_3)
  (`DecalComponent.SetDecalMaterial` (`self.Decal`) (`self.DecalMatInstance`)))

(event `self.ReceiveTick`
  (params (DeltaSeconds :type "Float (single-precision)"))
  (bind _decal (`self.Decal`))
  (bind _hitresult (`PlayerController.GetHitResultUnderCursorByChannel` (`GameplayStatics.GetPlayerController` 0) "TraceTypeQuery1" true))
  (bind ((`SculptRadius` _sculptradius) (`Falloff` _falloff)) (break `SculptSettings` (`SculptComponent.SculptSettings` (`self.Sculpt`))))
  (bind _returnvalue (/ _sculptradius 50.0))
  ;[1 1 1] Tick
  (`|ExecutionSequence`
    (:`then_0`
      ;;[1 1 1] IMPORTANT: necessary in order that the sculpt component works properly
      (set `self.CurrentHitLocation` _hitresult)
      (`SculptComponent.SetHitResult` (`self.Sculpt`) _hitresult)
      ;;[1 1 1] set brush decal location and size
      (`/Engine/EditorBlueprintResources/StandardMacros.IsValid` _decal
        (:`Is Valid`
          (`SceneComponent.K2_SetWorldLocation` _decal (`.Location` (`GameplayStatics.BreakHitResult` _hitresult)) false false)
          (`SceneComponent.SetWorldScale3D` _decal (`KismetMathLibrary.MakeVector` 500.0 _returnvalue _returnvalue))
          (`MaterialInstanceDynamic.SetScalarParameterValue` (`self.DecalMatInstance`) "InnerCircle" (- (/ _falloff 2.0) 0.01))
          (`SceneComponent.K2_SetWorldRotation` (`self.Decal`) (struct :`Pitch` -90.0) false false))))))

(fn `UserConstructionScript`)