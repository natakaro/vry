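; VR HUD actor with four spheres that show the player's Terrain, Bolt, Tree and Signal mana and act as the tool selector.
; Tick sets each sphere's material fill from mana and its color from selection and right-hand hover.
; Touch-sphere begin and end overlaps run TouchTest, which rumbles the controller and, for the right hand, sets the tool unless SculptSingle is active.
; BeginPlay attaches tree and signal actors; On/Off handle visibility and scale-in.
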(event `self.ReceiveTick`
  (params (DeltaSeconds :type "Float (single-precision)"))
  (bind _spheretree (`self.SphereTree`))
  (bind _player (`self.Player`))
  (bind _player_2 (`self.Player`))
  (bind _player_3 (`self.Player`))
  (bind _player_4 (`self.Player`))
  (bind _sphereterrain (`self.SphereTerrain`))
  (bind _spheresignal (`self.SphereSignal`))
  (`MeshComponent.SetScalarParameterValueOnMaterials` (`self.SphereTerrain`) "FillAmount" (/ (`/Game/Proteus_Single/Blueprints/MotionControllerPawn.manaTerrain` _player) (`/Game/Proteus_Single/Blueprints/MotionControllerPawn.maxMana` _player)))
  (`MeshComponent.SetScalarParameterValueOnMaterials` (`self.SphereBolt`) "FillAmount" (/ (`/Game/Proteus_Single/Blueprints/MotionControllerPawn.manaBolt` _player_2) (`/Game/Proteus_Single/Blueprints/MotionControllerPawn.maxMana` _player_2)))
  (`MeshComponent.SetScalarParameterValueOnMaterials` (`self.SphereTree`) "FillAmount" (/ (`/Game/Proteus_Single/Blueprints/MotionControllerPawn.manaTree` _player_3) (`/Game/Proteus_Single/Blueprints/MotionControllerPawn.maxMana` _player_3)))
  (`MeshComponent.SetScalarParameterValueOnMaterials` (`self.SphereSignal`) "FillAmount" (/ (`/Game/Proteus_Single/Blueprints/MotionControllerPawn.manaSignal` _player_4) (`/Game/Proteus_Single/Blueprints/MotionControllerPawn.maxMana` _player_4)))
  (`MeshComponent.SetVectorParameterValueOnMaterials` (`self.SphereTerrain`) "Color" (`self.colorInactive`))
  (`MeshComponent.SetVectorParameterValueOnMaterials` (`self.SphereBolt`) "Color" (`self.colorInactive`))
  (`MeshComponent.SetVectorParameterValueOnMaterials` (`self.SphereTree`) "Color" (`self.colorInactive`))
  (`MeshComponent.SetVectorParameterValueOnMaterials` (`self.SphereSignal`) "Color" (`self.colorInactive`))
  (`|ExecutionSequence`
    (:`then_0`
      (switch `/Game/Blueprints/tools` (`/Game/Proteus_Single/Blueprints/MotionControllerPawn.tools` (`self.Player`))
        (:`NewEnumerator0`
          (`MeshComponent.SetVectorParameterValueOnMaterials` (`self.SphereTerrain`) "Color" (`self.colorSelected`)))
        (:`NewEnumerator1`
          (`MeshComponent.SetVectorParameterValueOnMaterials` (`self.SphereTree`) "Color" (`self.colorSelected`)))
        (:`NewEnumerator2`
          (`MeshComponent.SetVectorParameterValueOnMaterials` (`self.SphereSignal`) "Color" (`self.colorSelected`)))
        (:`NewEnumerator3`
          (`MeshComponent.SetVectorParameterValueOnMaterials` (`self.SphereBolt`) "Color" (`self.colorSelected`)))))
    (:`then_1`
      (if (`PrimitiveComponent.IsOverlappingComponent` _spheresignal (`/Game/Proteus_Single/Blueprints/BP_MotionController.TouchSphere` (`/Game/Proteus_Single/Blueprints/MotionControllerPawn.RightController` (`self.Player`))))
        (`MeshComponent.SetVectorParameterValueOnMaterials` _spheresignal "Color" (`self.colorHover`))
        (elif (`PrimitiveComponent.IsOverlappingComponent` _spheretree (`/Game/Proteus_Single/Blueprints/BP_MotionController.TouchSphere` (`/Game/Proteus_Single/Blueprints/MotionControllerPawn.RightController` (`self.Player`))))
          (`MeshComponent.SetVectorParameterValueOnMaterials` _spheretree "Color" (`self.colorHover`))
          (elif (`PrimitiveComponent.IsOverlappingComponent` (`self.SphereBolt`) (`/Game/Proteus_Single/Blueprints/BP_MotionController.TouchSphere` (`/Game/Proteus_Single/Blueprints/MotionControllerPawn.RightController` (`self.Player`))))
            (if (`PrimitiveComponent.IsOverlappingComponent` _sphereterrain (`/Game/Proteus_Single/Blueprints/BP_MotionController.TouchSphere` (`/Game/Proteus_Single/Blueprints/MotionControllerPawn.RightController` (`self.Player`))))
              (`MeshComponent.SetVectorParameterValueOnMaterials` _sphereterrain "Color" (`self.colorHover`)))))))))

(event `self.ReceiveBeginPlay`
  (`self.SpawnTree`)
  (`self.SpawnSignal`))

(event `self.SphereTerrain.OnComponentBeginOverlap`
  (params (OverlappedComponent :type "PrimitiveComponent Object Reference") (OtherActor :type "Actor Object Reference") (OtherComp :type "PrimitiveComponent Object Reference") (OtherBodyIndex :type Integer) (bFromSweep :type Boolean) (SweepResult :type "HitResult Structure (by ref)"))
  (`self.TouchTest` OtherActor OtherComp "NewEnumerator0"))

(event `self.Sphere.OnComponentBeginOverlap`
  (params (OverlappedComponent :type "PrimitiveComponent Object Reference") (OtherActor :type "Actor Object Reference") (OtherComp :type "PrimitiveComponent Object Reference") (OtherBodyIndex :type Integer) (bFromSweep :type Boolean) (SweepResult :type "HitResult Structure (by ref)")))

(event `self.SphereTree.OnComponentBeginOverlap`
  (params (OverlappedComponent :type "PrimitiveComponent Object Reference") (OtherActor :type "Actor Object Reference") (OtherComp :type "PrimitiveComponent Object Reference") (OtherBodyIndex :type Integer) (bFromSweep :type Boolean) (SweepResult :type "HitResult Structure (by ref)"))
  (`self.TouchTest` OtherActor OtherComp "NewEnumerator1"))

(event `self.SphereSignal.OnComponentBeginOverlap`
  (params (OverlappedComponent :type "PrimitiveComponent Object Reference") (OtherActor :type "Actor Object Reference") (OtherComp :type "PrimitiveComponent Object Reference") (OtherBodyIndex :type Integer) (bFromSweep :type Boolean) (SweepResult :type "HitResult Structure (by ref)"))
  (`self.TouchTest` OtherActor OtherComp "NewEnumerator2"))

(event `self.StaticMesh2.OnComponentBeginOverlap`
  (params (OverlappedComponent :type "PrimitiveComponent Object Reference") (OtherActor :type "Actor Object Reference") (OtherComp :type "PrimitiveComponent Object Reference") (OtherBodyIndex :type Integer) (bFromSweep :type Boolean) (SweepResult :type "HitResult Structure (by ref)")))

(event `self.StaticMesh3.OnComponentBeginOverlap`
  (params (OverlappedComponent :type "PrimitiveComponent Object Reference") (OtherActor :type "Actor Object Reference") (OtherComp :type "PrimitiveComponent Object Reference") (OtherBodyIndex :type Integer) (bFromSweep :type Boolean) (SweepResult :type "HitResult Structure (by ref)")))

(event `self.SphereBolt.OnComponentBeginOverlap`
  (params (OverlappedComponent :type "PrimitiveComponent Object Reference") (OtherActor :type "Actor Object Reference") (OtherComp :type "PrimitiveComponent Object Reference") (OtherBodyIndex :type Integer) (bFromSweep :type Boolean) (SweepResult :type "HitResult Structure (by ref)"))
  (`self.TouchTest` OtherActor OtherComp "NewEnumerator3"))

(event `self.SphereTree.OnComponentEndOverlap`
  (params (OverlappedComponent :type "PrimitiveComponent Object Reference") (OtherActor :type "Actor Object Reference") (OtherComp :type "PrimitiveComponent Object Reference") (OtherBodyIndex :type Integer))
  (`self.TouchTest` OtherActor OtherComp "NewEnumerator1"))

(event `self.SphereSignal.OnComponentEndOverlap`
  (params (OverlappedComponent :type "PrimitiveComponent Object Reference") (OtherActor :type "Actor Object Reference") (OtherComp :type "PrimitiveComponent Object Reference") (OtherBodyIndex :type Integer))
  (`self.TouchTest` OtherActor OtherComp "NewEnumerator2"))

(event `self.SphereBolt.OnComponentEndOverlap`
  (params (OverlappedComponent :type "PrimitiveComponent Object Reference") (OtherActor :type "Actor Object Reference") (OtherComp :type "PrimitiveComponent Object Reference") (OtherBodyIndex :type Integer))
  (`self.TouchTest` OtherActor OtherComp "NewEnumerator3"))

(event `self.SphereTerrain.OnComponentEndOverlap`
  (params (OverlappedComponent :type "PrimitiveComponent Object Reference") (OtherActor :type "Actor Object Reference") (OtherComp :type "PrimitiveComponent Object Reference") (OtherBodyIndex :type Integer))
  (`self.TouchTest` OtherActor OtherComp "NewEnumerator0"))

(fn `Off`
  (`SceneComponent.SetVisibility` (`self.DefaultSceneRoot`) false true))

(fn `On`
  (bind _defaultsceneroot (`self.DefaultSceneRoot`))
  (if (`SceneComponent.IsVisible` (`self.DefaultSceneRoot`))
    (`SceneComponent.SetWorldScale3D` _defaultsceneroot (`KismetMathLibrary.Conv_DoubleToVector` (`KismetMathLibrary.Lerp` 0.0 10.0 (`KismetMathLibrary.FClamp` (* (- (`GameplayStatics.GetTimeSeconds`) (`self.startTime`)) 4.0)))))
    (else
      (`SceneComponent.SetWorldScale3D` (`self.DefaultSceneRoot`) (0.0 0.0 0.0))
      (set `self.startTime` (`GameplayStatics.GetTimeSeconds`))
      (`SceneComponent.SetVisibility` _defaultsceneroot true true))))

(fn `Rumble`
  (params (Controller :type "/Game/Proteus_Single/Blueprints/BP_MotionController Object Reference"))
  (`/Game/Proteus_Single/Blueprints/BP_MotionController.RumbleController` Controller 0.8))

(fn `SpawnSignal`
  (bind _returnvalue (`|SpawnActorFromClass` "/Game/Blueprints/Sig.Sig_C" (`KismetMathLibrary.MakeTransform` (0.0 0.0 0.0)) "Undefined" "OverrideRootScale" null self))
  (`self.K2_AttachToComponent` _returnvalue (`self.Sphere1`) "None" "SnapToTarget" "SnapToTarget" "KeepWorld" false)
  (set `self.signalActor` _returnvalue))

(fn `SpawnTree`
  (bind _returnvalue (`|SpawnActorFromClass` "/Game/Blueprints/tree.tree_C" (`KismetMathLibrary.MakeTransform` (0.0 0.0 0.0)) "Undefined" "OverrideRootScale" null self))
  (`self.K2_AttachToComponent` _returnvalue (`self.Sphere`) "None" "SnapToTarget" "SnapToTarget" "KeepWorld" false)
  (set `self.treeActor` _returnvalue))

(fn `UserConstructionScript`)