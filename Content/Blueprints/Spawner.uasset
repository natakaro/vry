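; Spawner actor that scatters randomly chosen actors from a class array across a large area of the world.
; On BeginPlay it calls Reset, which waits briefly, then loops N times, line tracing between random high and low points against WorldStatic to find a location.
; A sphere overlap check rejects spots near dynamic objects, pawns or a custom object type; otherwise it spawns there and prints the actor's name.
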(event `self.ReceiveBeginPlay`
  (`self.Reset`))

(event `Reset`
  (bind _returnvalue (`KismetMathLibrary.RandomFloatInRange` 10000.0 80000.0))
  (bind _returnvalue_2 (`KismetMathLibrary.RandomFloatInRange` 10000.0 80000.0))
  (bind _arrayofclass (`self.ArrayOfClass`))
  (`KismetSystemLibrary.Delay` 5.0)
  (for _ (range (+ (`self.N`) 1))
    (bind _outhit (`KismetSystemLibrary.LineTraceSingleForObjects` :`Start` (`KismetMathLibrary.MakeVector` _returnvalue_2 _returnvalue 100000.0) :`End` (`KismetMathLibrary.MakeVector` _returnvalue_2 _returnvalue -1000.0) :`ObjectTypes` (`|MakeArray` "ObjectTypeQuery1" :!type "EObjectTypeQuery Enum") :`DrawDebugType` "ForOneFrame"))
    (bind (_bblockinghit _binitialoverlap _time _location) (`GameplayStatics.BreakHitResult` _outhit))
    (bind (_outhits _returnvalue_3) (`KismetSystemLibrary.SphereTraceMultiForObjects` _location _location 500.0 (`|MakeArray` "ObjectTypeQuery2" "ObjectTypeQuery3" "ObjectTypeQuery8" :!type "EObjectTypeQuery Enum")))
    (if (not _returnvalue_3)
      (bind _returnvalue_4 (`|SpawnActorFromClass` (`KismetArrayLibrary.Array_Get` _arrayofclass (`KismetMathLibrary.RandomInteger` (`KismetArrayLibrary.Array_Length` _arrayofclass))) (`KismetMathLibrary.MakeTransform` _location) "Undefined" "OverrideRootScale"))
      (`KismetSystemLibrary.PrintString` (`KismetSystemLibrary.GetDisplayName` _returnvalue_4) true true (struct :`G` 0.66 :`B` 1.0 :`A` 1.0) 5.0))))

(fn `UserConstructionScript`)